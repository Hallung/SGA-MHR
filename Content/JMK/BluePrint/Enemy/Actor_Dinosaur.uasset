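; Dinosaur enemy character driven by a behavior tree AI controller, with hit reactions and death.
; On spawn it stores its start position and caches the BT_Controller.
; Damage reduces health through the monster stat component and mirrors hit and dead states to the blackboard, playing a timed hit montage, or a death montage before disabling collision and destroying itself after a delay.
; Helper functions expose the start position, attack flag and attack distance selection.
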(event Collision|EventActorBeginOverlap
  (params (OtherActor :type Actor%20Object%20Reference)))

(event EventTick
  (params (DeltaSeconds :type Float%20%28single-precision%29)))

(event Game|Damage|EventAnyDamage
  (params (Damage :type Float%20%28single-precision%29) (DamageType :type Damage%20Type%20Object%20Reference) (InstigatedBy :type Controller%20Object%20Reference) (DamageCauser :type Actor%20Object%20Reference))
  (bind _output_get (Variables|Default|SetIsHit true))
  (Default|SetBBIsHit (Variables|Default|GetBT_Controller) _output_get)
  (Variables|Default|SetDamage%20Causer DamageCauser)
  (bind _isdead (Default|DecreaseHealth (Variables|Default|GetBPC_MonsterStatSystem) Damage))
  (bind _output_get_2 (Variables|Default|SetIsDead _isdead))
  (if _output_get_2
    (Default|SetBBIsDead (Variables|Default|GetBT_Controller) (Variables|Default|GetIsDead))
    (Animation|PlayAnimMontage "/Game/CustomContents/Monster/Small/Izuchi/Animation/Damage/Montage/dead_Montage.dead_Montage" 1.0 "None")
    (Collision|SetCollisionEnabled (Variables|Collision|GetCapsuleComponent) "NoCollision")
    (Utilities|FlowControl|Delay 1e+01)
    (Actor|DestroyActor)
    (else
      (bind _returnvalue (Animation|PlayAnimMontage "/Game/CustomContents/Monster/Small/Izuchi/Animation/Damage/Montage/damage_front_Montage.damage_front_Montage" 1.0 "None"))
      (Utilities|FlowControl|Delay _returnvalue)
      (bind _output_get_3 (Variables|Default|SetIsHit false))
      (Default|SetBBIsHit (Variables|Default|GetBT_Controller) _output_get_3))))

(event EventBeginPlay
  (Variables|Default|SetInitPos (Transformation|GetActorLocation))
  (bind _asai_컨트롤러 (Utilities|Casting|CastToAIController (Pawn|GetController)))
  (bind _asbt_controller (Utilities|Casting|CastToBT_Controller _asai_컨트롤러))
  (Variables|Default|SetBT_Controller _asbt_controller))

(fn ConstructionScript)

(fn GetInitPos
  (return (Variables|Default|GetInitPos)))

(fn SetAttackBool
  (params (Value :type Boolean))
  ;[0.15 0.15 0.15 0.5] Anim의 Attack 제어하는 Bool값
  (Variables|Default|SetCanAttack Value))

(fn SetCurAttackDist
  (params (Index :type Integer))
  (Variables|Default|SetCurAttackDist (Utilities|Array|Get(acopy) (Variables|Default|GetAttackDistArray) Index)))