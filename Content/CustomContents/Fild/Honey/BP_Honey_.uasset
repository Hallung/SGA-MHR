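; BP_Honey_ is a honey item that reappears after being hidden and shows a widget when something is within range.
; Tick starts a 60-second Delay while the Honey2 component is hidden, then makes it visible again.
; Sphere overlaps set the Can flag and toggle the widget, which appears only while honey is visible, with no filter on the overlapping actor.
; The construction script sets the item type and name enums.
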(event OnComponentBeginOverlap(Sphere)
  (params (OverlappedComponent :type Primitive%20Component%20Object%20Reference) (OtherActor :type Actor%20Object%20Reference) (OtherComp :type Primitive%20Component%20Object%20Reference) (OtherBodyIndex :type Integer) (bFromSweep :type Boolean) (SweepResult :type Hit%20Result%20Structure%20%28by%20ref%29))
  (if (Variables|/Script/Engine.SceneComponent|GetbVisible (Variables|Default|GetHoney2))
    (Variables|Default|SetCan true)
    (Rendering|SetVisibility (Variables|Default|GetWidget) true false)
    (else
      (Variables|Default|SetCan true))))

(event OnComponentEndOverlap(Sphere)
  (params (OverlappedComponent :type Primitive%20Component%20Object%20Reference) (OtherActor :type Actor%20Object%20Reference) (OtherComp :type Primitive%20Component%20Object%20Reference) (OtherBodyIndex :type Integer))
  (Variables|Default|SetCan false)
  (Rendering|SetVisibility (Variables|Default|GetWidget) false false))

(event EventTick
  (params (DeltaSeconds :type Float%20%28single-precision%29))
  (if (not (Variables|/Script/Engine.SceneComponent|GetbVisible (Variables|Default|GetHoney2)))
    (Utilities|FlowControl|Delay 6e+01)
    (Rendering|SetVisibility (Variables|Default|GetHoney2) true false)
    (if (Variables|Default|GetCan)
      (Rendering|SetVisibility (Variables|Default|GetWidget) true false)
      (else
        (Rendering|SetVisibility (Variables|Default|GetWidget) false false)))))

(fn ConstructionScript
  (|CallParentFunction)
  (Variables|Default|SetItemType "NewEnumerator1")
  (Variables|Default|SetItemName "NewEnumerator0"))