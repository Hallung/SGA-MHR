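; BP_Exit is an exit marker that shows a widget while something overlaps its sphere trigger.
; The widget appears on begin overlap only when the game instance's QuestNum is non-zero, and hides on end overlap, with no check on which actor overlaps.
; On BeginPlay it tries to cache its owner as a BP_HallPlayerCharacter, but neither overlap event uses that reference.
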(event OnComponentBeginOverlap(Sphere)
  (params (OverlappedComponent :type Primitive%20Component%20Object%20Reference) (OtherActor :type Actor%20Object%20Reference) (OtherComp :type Primitive%20Component%20Object%20Reference) (OtherBodyIndex :type Integer) (bFromSweep :type Boolean) (SweepResult :type Hit%20Result%20Structure%20%28by%20ref%29))
  (bind _asbp_game_instance (Utilities|Casting|CastToBP_GameInstance (Game|GetGameInstance)))
  (if (!= (Variables|/Game/CustomContents/GameInstance/BP_GameInstance.BP_GameInstance_C|GetQuestNum _asbp_game_instance) 0)
    (Rendering|SetVisibility (Variables|Default|GetWidget) true false)))

(event OnComponentEndOverlap(Sphere)
  (params (OverlappedComponent :type Primitive%20Component%20Object%20Reference) (OtherActor :type Actor%20Object%20Reference) (OtherComp :type Primitive%20Component%20Object%20Reference) (OtherBodyIndex :type Integer))
  (Rendering|SetVisibility (Variables|Default|GetWidget) false false))

(event EventBeginPlay
  (bind _asbp_hall_player_character (Utilities|Casting|CastToBP_HallPlayerCharacter (Components|GetOwner)))
  (Variables|Default|SetBP%20Hall%20Player%20Character _asbp_hall_player_character))

(fn ConstructionScript)