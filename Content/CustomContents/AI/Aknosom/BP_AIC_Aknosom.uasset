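; AI controller for the Aknosom monster that runs its behavior tree and manages aggro and battle music.
; Pawn sensing records the last sighting time, writes the seen pawn to the blackboard and starts battle music, unless Aknosom is running away.
; A looping timer polls the time since the last sighting, clearing the target and battle blackboard keys and fading the music after the aggro release time.
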(event OnSeePawn(PawnSensing)
  (params (Pawn :type Pawn%20Object%20Reference))
  (bind _asbp_aknosom (Utilities|Casting|CastToBP_Aknosom (Pawn|GetControlledPawn)))
  (if (not (Variables|/Game/CustomContents/Monster/Boss/BP_Aknosom.BP_Aknosom_C|GetIsRunAway _asbp_aknosom))
    (Variables|Default|SetLastSeenTime (Utilities|Time|GetGameTimeinSeconds))
    (AI|Components|Blackboard|SetValueasBool (AI|GetBlackboard 0) (Utilities|Name|MakeLiteralName "SeeingTarget?") true)
    (AI|Components|Blackboard|SetValueasObject (AI|GetBlackboard 0) (Utilities|Name|MakeLiteralName "Player") Pawn)
    (Utilities|IsValid (Variables|Default|GetBattleBGM)
      (:Is%20Valid
        _)
      (:Is%20Not%20Valid
        (bind _returnvalue (Audio|SpawnSound2D "/Game/CustomContents/Sound/BGM/magnamalo_Battle.magnamalo_Battle" 1.0 1.0 0.0 0))
        (Variables|Default|SetBattleBGM _returnvalue)))
    (Utilities|Time|SetTimerbyFunctionName 0 "CheckAggroTimeout" 0.5 true)))

(event EventBeginPlay
  (AI|RunBehaviorTree "/Game/CustomContents/AI/Aknosom/BT_Aknosom.BT_Aknosom"))

(fn ConstructionScript)

(fn CheckAggroTimeout
  (bind _battlebgm (Variables|Default|GetBattleBGM))
  (if (> (- (Utilities|Time|GetGameTimeinSeconds) (Variables|Default|GetLastSeenTime)) (Variables|Default|GetAggroReleaseTime))
    (AI|Components|Blackboard|ClearValue (AI|GetBlackboard 0) (Utilities|Name|MakeLiteralName "SeeingTarget?"))
    (AI|Components|Blackboard|ClearValue (AI|GetBlackboard 0) (Utilities|Name|MakeLiteralName "Player"))
    (AI|Components|Blackboard|ClearValue (AI|GetBlackboard 0) (Utilities|Name|MakeLiteralName "IsBattle"))
    (Utilities|IsValid _battlebgm
      (:Is%20Valid
        (Audio|Components|Audio|FadeOut _battlebgm 2.0 0.0 "Linear" :!class /Script/Engine.AudioComponent)))))