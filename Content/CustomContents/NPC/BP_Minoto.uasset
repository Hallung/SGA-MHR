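; BP_Minoto is an NPC Blueprint that shows a widget component while something is within its sphere trigger.
; On BeginPlay it caches the mesh's ABP_Minoto anim instance and, if that cast succeeds, resets its Interaction flag to false.
; Sphere begin and end overlap toggle the widget's visibility, with no check on which actor overlaps.
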(event OnComponentBeginOverlap(Sphere)
  (params (OverlappedComponent :type Primitive%20Component%20Object%20Reference) (OtherActor :type Actor%20Object%20Reference) (OtherComp :type Primitive%20Component%20Object%20Reference) (OtherBodyIndex :type Integer) (bFromSweep :type Boolean) (SweepResult :type Hit%20Result%20Structure%20%28by%20ref%29))
  (Rendering|SetVisibility (Variables|Default|GetWidget) true false))

(event OnComponentEndOverlap(Sphere)
  (params (OverlappedComponent :type Primitive%20Component%20Object%20Reference) (OtherActor :type Actor%20Object%20Reference) (OtherComp :type Primitive%20Component%20Object%20Reference) (OtherBodyIndex :type Integer))
  (Rendering|SetVisibility (Variables|Default|GetWidget) false false))

(event EventBeginPlay
  (bind _asabp_minoto (Utilities|Casting|CastToABP_Minoto (Components|SkeletalMesh|GetAnimInstance (Variables|Character|GetMesh))))
  (Variables|Default|SetABP%20Minoto _asabp_minoto)
  (Variables|Default|SetInteraction false))

(fn ConstructionScript)