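; Training variant of the Izuchi small monster that detects the player, attacks and reacts to being hit.
; A detector overlap stores the player character and passes it to the training AI controller as the target.
; Damage plays a hit montage and holds a blackboard hit flag for its duration.
; StartAttack sets a timer for a head sphere trace that damages the hit actor unless the player is dead; StopAttack clears it.
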(event OnComponentBeginOverlap(TempDetector)
  (params (OverlappedComponent :type Primitive%20Component%20Object%20Reference) (OtherActor :type Actor%20Object%20Reference) (OtherComp :type Primitive%20Component%20Object%20Reference) (OtherBodyIndex :type Integer) (bFromSweep :type Boolean) (SweepResult :type Hit%20Result%20Structure%20%28by%20ref%29))
  (bind _asbp_player_character (Utilities|Casting|CastToBP_PlayerCharacter OtherActor))
  (Variables|Default|SetPlayer%20Character _asbp_player_character)
  (bind _asaic_monster_training (Utilities|Casting|CastToAIC_Monster_Training (AI|GetAIController self)))
  (Default|SetTarget _asaic_monster_training _asbp_player_character))

(event Custom|StartAttack
  (bind _returnvalue (Utilities|Time|SetTimerbyEvent (delegate Custom|Attack) 0.01))
  (Variables|Default|SetAttackTimerHandler _returnvalue))

(event Custom|Attack
  (bind (_outhit _returnvalue) (Collision|SphereTraceForObjects (Transformation|GetWorldLocation (Variables|Default|GetHeadStart)) (Transformation|GetWorldLocation (Variables|Default|GetHeadEnd)) 3e+01 (Utilities|Array|MakeArray "ObjectTypeQuery10" "ObjectTypeQuery9" "ObjectTypeQuery11") false 0 "None" true "(R=1.000000,G=0.000000,B=0.000000,A=1.000000)" "(R=0.000000,G=1.000000,B=0.000000,A=1.000000)" 0.5))
  (if _returnvalue
    (if (not (Variables|/Game/CustomContents/Components/BPC_PlayerStatSystem.BPC_PlayerStatSystem_C|GetIsDead (Variables|/Game/CustomContents/Player/BP_PlayerCharacter.BP_PlayerCharacter_C|GetBPC_PlayerStatSystem (Variables|Default|GetPlayer%20Character))))
      (Game|Damage|ApplyDamage (.HitActor (Collision|BreakHitResult _outhit)) 5.0 0 self))))

(event Custom|StopAttack
  (Utilities|Time|ClearandInvalidateTimerbyHandle (Variables|Default|GetAttackTimerHandler)))

(event EventBeginPlay
  (bind _asabp_izuchi (Utilities|Casting|CastToABP_Izuchi (Components|SkeletalMesh|GetAnimInstance (Variables|Character|GetMesh))))
  (Variables|Default|SetAnimationBP _asabp_izuchi))

(event Game|Damage|EventAnyDamage
  (params (Damage :type Float%20%28single-precision%29) (DamageType :type Damage%20Type%20Object%20Reference) (InstigatedBy :type Controller%20Object%20Reference) (DamageCauser :type Actor%20Object%20Reference))
  (bind _output_get (Variables|Default|SetIsHit true))
  (AI|Components|Blackboard|SetValueasBool (AI|GetBlackboard 0) (Variables|Default|GetIsHitBlackboardKey) _output_get)
  (bind _returnvalue (Animation|PlayAnimMontage "/Game/CustomContents/Monster/Small/Izuchi/Animation/Damage/Montage/damage_front_Montage.damage_front_Montage" 1.0 "None"))
  (Utilities|FlowControl|Delay _returnvalue)
  (bind _output_get_2 (Variables|Default|SetIsHit false))
  (AI|Components|Blackboard|SetValueasBool (AI|GetBlackboard 0) (Variables|Default|GetIsHitBlackboardKey) _output_get_2))

(fn ConstructionScript)