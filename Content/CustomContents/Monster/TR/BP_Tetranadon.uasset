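; BP_Tetranadon is a monster that plays field battle music and an idle sound when play begins.
; Its attack starts a fast looping timer that sphere-traces between the Start and End mesh sockets until stopped.
; A DamagedPlayer list limits each target to one hit per attack and is cleared on stop.
; Hit players are launched horizontally away before taking delayed random damage, while other actors take it immediately.
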(event Custom|StartTRAttack
  (bind _returnvalue (Utilities|Time|SetTimerbyEvent (delegate Custom|TRAttackTrace) 0.01 true))
  (Variables|Default|SetTRAttackHandle _returnvalue))

(event Custom|TRAttackTrace
  (|TRAttack))

(event Custom|StopTRAttackTrace
  (Utilities|Time|ClearandInvalidateTimerbyHandle (Variables|Default|GetTRAttackHandle))
  (Utilities|Array|Clear (Variables|Default|GetDamagedPlayer)))

(event EventBeginPlay
  (bind _returnvalue (Audio|SpawnSound2D "/Game/CustomContents/Sound/BGM/FildBattle.FildBattle" 1.0 1.0 0.0 0))
  (Variables|Default|SetTRBGM _returnvalue)
  (Audio|SpawnSoundatLocation "/Game/CustomContents/Sound/TR/Idle.Idle" (Transformation|GetActorLocation) "0, 0, 0" 1.0 1.0 0.0 0 0))

(fn ConstructionScript)